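; Quad damage powerup that temporarily quadruples the weapon damage of the player who activates it.
; On activation it stores the player and multiplies BaseDamage on their CSCharacter's CurrentWeapon by four, then calls the parent handler.
; On expiry it divides BaseDamage by four on whichever weapon is current at that moment, then calls the parent handler.
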(event `self.OnActivated`
  (params (ActiveFor :type "Actor Object Reference"))
  (bind _output_get (set `self.ActivateForPlayer` ActiveFor))
  (bind _ascscharacter (cast `CSCharacter` _output_get))
  (bind _currentweapon (`CSCharacter.CurrentWeapon` _ascscharacter))
  (set `CSWeapon.BaseDamage` (* (`CSWeapon.BaseDamage` _currentweapon) 4.0) _currentweapon)
  (`parent.OnActivated` null))

(event `self.OnExpired`
  (bind _ascscharacter (cast `CSCharacter` (`self.ActivateForPlayer`)))
  (bind _currentweapon (`CSCharacter.CurrentWeapon` _ascscharacter))
  (set `CSWeapon.BaseDamage` (/ (`CSWeapon.BaseDamage` _currentweapon) 4.0) _currentweapon)
  (`parent.OnExpired`))

(fn `UserConstructionScript`
  (`parent.UserConstructionScript`))