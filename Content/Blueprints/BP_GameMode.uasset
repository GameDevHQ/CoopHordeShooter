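; Game mode Blueprint that spawns AI bots and awards score for killing them.
; SpawnNewBot runs an EQS query for spawn locations, then spawns either an advanced AI or a tracker bot, chosen at random, at the returned locations.
; An OnActorKilled binding made at BeginPlay adds fixed points to the killer's CSPlayerState when a non-player pawn dies, then prints the score.
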(event `self.SpawnNewBot`
  (bind _returnvalue (`EnvQueryManager.RunEQSQuery` "/Game/Blueprints/EQS/EQS_FindSpawnLocation.EQS_FindSpawnLocation" self "RandomBest25Pct"))
  (add `EnvQueryInstanceBlueprintWrapper.OnQueryFinishedEvent` _returnvalue (delegate `OnQueryFinishedEvent_Event_0`)))

(event `OnQueryFinishedEvent_Event_0`
  (params (QueryInstance :type "EnvQueryInstanceBlueprintWrapper Object Reference") (QueryStatus :type "EEnvQueryStatus Enum" :default "Processing"))
  (switch `EEnvQueryStatus` QueryStatus
    (:`Success`
      (for _array_element (`EnvQueryInstanceBlueprintWrapper.GetResultsAsLocations` QueryInstance)
        (`|SpawnActorFromClass` (select `bool` (<= (`KismetMathLibrary.RandomIntegerInRange` 0 100) 50) :`false` "/Game/AI/TrackerBot/BP_TrackerBot.BP_TrackerBot_C" :`true` "/Game/AI/AdvancedAI/BP_AdvancedAI.BP_AdvancedAI_C" :!type "Actor Class Reference") (`KismetMathLibrary.MakeTransform` _array_element) "AdjustIfPossibleButDontSpawnIfColliding" "OverrideRootScale" null null)))))

(event `self.ReceiveBeginPlay`
  (add `self.OnActorKilled` (delegate `OnActorKilled_Event_0`)))

(event `OnActorKilled_Event_0` :!signature `self.OnActorKilled`
  (params (VictimActor :type "Actor Object Reference") (KillerActor :type "Actor Object Reference") (KillerController :type "Controller Object Reference"))
  (bind _playerstate (`Pawn.PlayerState` (`Controller.K2_GetPawn` KillerController)))
  (bind _aspawn (cast `Pawn` VictimActor))
  (if (not (`Pawn.IsPlayerControlled` _aspawn))
    (bind _ascsplayer_state (cast `CSPlayerState` _playerstate))
    (`CSPlayerState.AddScore` _ascsplayer_state 20.0)
    (`KismetSystemLibrary.PrintString` (`KismetStringLibrary.Conv_DoubleToString` (`PlayerState.Score` _playerstate)) true true (struct :`R` 0.017724 :`G` 1.0 :`B` 0.363362 :`A` 1.0))))

(fn `UserConstructionScript`)